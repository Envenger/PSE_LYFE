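; Grenade projectile actor that explodes after a short random fuse started on BeginPlay.
; A short downward trace picks the explosion emitter by indexing a list with the hit surface's physical material type, or uses an air burst on a miss.
; It then hides itself, places a scorch decal, shakes the camera and applies radial damage at the trace hit location, plus a one-time force impulse and sound.
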(event EventBeginPlay
  (bind _spherecollision (Variables|Default|GetSphereCollision))
  (bind _returnvalue (Transformation|GetWorldLocation _spherecollision))
  ;[1 1 1] Grenade Projectile Info
  (Variables|Default|SetGrenadeList (Utilities|Array|MakeArray (Variables|VFX|GetDefault) (Variables|VFX|GetConcrete) (Variables|VFX|GetDirt) (Variables|VFX|GetGrass) (Variables|VFX|GetIce) (Variables|VFX|GetMetal) (Variables|VFX|GetSand) (Variables|VFX|GetSnow) (Variables|VFX|GetWater) (Variables|VFX|GetWood)))
  (Variables|Default|SetFuseTime (Math|Random|RandomFloatinRange 1.0 2.0))
  (Variables|Default|SetArmed true)
  (Utilities|FlowControl|Delay (Variables|Default|GetFuseTime))
  (bind (_outhit _returnvalue_2) (Collision|LineTraceByChannel _returnvalue (+ _returnvalue "0, 0,-100.000000") "TraceTypeQuery1" false 0 "None"))
  (if _returnvalue_2
    (Effects|SpawnEmitteratLocation (Utilities|Array|Get(acopy) (Variables|Default|GetGrenadeList) (Math|Conversions|ToInteger(Byte) (Variables|/Script/Engine.PhysicalMaterial|GetSurfaceType (.PhysMat (Collision|BreakHitResult _outhit))))) (.Location (Collision|BreakHitResult _outhit)) (Math|Rotator|MakeRotationfromAxes (.Normal (Collision|BreakHitResult _outhit)) "0, 0, 0" "0, 0, 0"))
    (else
      (Effects|SpawnEmitteratLocation (Variables|VFX|GetAir) _returnvalue)))
  (bind _returnvalue_3 (Rendering|Decal|SpawnDecalatLocation "/Game/GrenadePack/Materials/M_scorch.M_scorch" "200.000000,200.000000,200.000000" (.Location (Collision|BreakHitResult _outhit)) "-90.000000,0.000000,0.000000" 0.0))
  (Rendering|SetActorHiddenInGame true)
  (Camera|PlayWorldCameraShake (Variables|Default|GetCameraShake) (.Location (Collision|BreakHitResult _outhit)) 0.0 2e+03)
  (Game|Damage|ApplyRadialDamage 2e+02 (.Location (Collision|BreakHitResult _outhit)) 1e+02 0 0 0 0 false "ECC_Visibility")
  (Utilities|FlowControl|DoOnce false
    (:Completed
      (Class|RadialForceComponent|FireImpulse (Variables|Default|GetRadialForce1))
      (Class|GameplayStatics|PlaySoundAttached "/Game/Audio/Explosion01.Explosion01" _returnvalue_3))))

(fn ConstructionScript)